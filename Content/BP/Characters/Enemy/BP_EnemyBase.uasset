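; Base enemy Blueprint that uses the Gameplay Ability System and triggers a roguelite level-up choice when it dies.
; On BeginPlay it applies a startup gameplay effect, and damage events spawn normal or critical damage widgets through DamageHandler.
; Death sets a short lifespan, disables damage widgets and queries the roguelite subsystem's level-up pool.
; Any results open a selection widget that pauses the game until the chosen action is acquired.
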(event Custom|OnSelectAction_Event
  (params (SelectedAction :type BP%20Runner%20Action%20Data%20Object%20Reference))
  (bind _returnvalue (Game|GetPlayerController 0))
  (Class|RogueliteSubsystem|AcquireAction (Subsystems|GetRogueliteSubsystem) SelectedAction 1)
  (Widget|RemovefromParent (Variables|Default|GetSelectionWidget))
  (Input|SetInputModeGameOnly _returnvalue false)
  (Variables|/Script/Engine.PlayerController|SetbShowMouseCursor _returnvalue false)
  (Game|SetGamePaused false))

(event EventBeginPlay
  (GameplayEffects|ApplyGameplayEffectSpecToSelf (Variables|Default|GetAbilitySystemComponent) (GameplayEffects|MakeOutgoingSpec (Variables|Default|GetAbilitySystemComponent) (Variables|Default|GetStartupEffect) 0.0 (GameplayEffects|MakeEffectContext (Variables|Default|GetAbilitySystemComponent)))))

(event EventOnDamageApplied
  (params (DamageAmount :type Float%20%28single-precision%29) (bIsCriticalHit :type Boolean))
  (bind _damagehandler (Variables|Default|GetDamageHandler))
  (if bIsCriticalHit
    (Default|SpawnDamageWidget _damagehandler "NewEnumerator1" DamageAmount)
    (else
      (Default|SpawnDamageWidget _damagehandler "NewEnumerator0" DamageAmount))))

(event EventDie
  (bind _returnvalue (Game|GetPlayerController 0))
  (Variables|Default|SetbIsDead true)
  (Actor|SetLifeSpan 1.0)
  (Variables|/Game/BP/Combat/BP_DamageHandler.BP_DamageHandler_C|SetEnableSpawnWidget (Variables|Default|GetDamageHandler) false)
  (bind _returnvalue_2 (Class|RogueliteSubsystem|ExecuteQuery (Subsystems|GetRogueliteSubsystem) (Utilities|Struct|MakeRogueliteQuery 0 "(GameplayTags=((TagName=\"Pool.LevelUp\")))")))
  (if (not (Utilities|Array|IsEmpty _returnvalue_2))
    (bind _returnvalue_3 (UserInterface|CreateWidget "/Game/BP/UI/Temp/W_SelectAction.W_SelectAction_C"))
    (Variables|Default|SetSelectionWidget _returnvalue_3)
    (Default|SetSelections (Variables|Default|GetSelectionWidget) _returnvalue_2)
    (EventDispatchers|AssignOnSelectAction (Variables|Default|GetSelectionWidget) (delegate Custom|OnSelectAction_Event))
    (Game|SetGamePaused true)
    (UserInterface|Viewport|AddtoViewport (Variables|Default|GetSelectionWidget) 0)
    (Input|SetInputModeUIOnly _returnvalue (Variables|Default|GetSelectionWidget) "DoNotLock" false)
    (Variables|/Script/Engine.PlayerController|SetbShowMouseCursor _returnvalue true)))

(fn ConstructionScript)

(fn IsDead
  (return (Variables|Default|GetbIsDead)))