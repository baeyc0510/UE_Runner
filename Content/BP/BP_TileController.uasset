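; BP_TileController builds an endlessly recycled track of BP_Tile actors along the X axis.
; On BeginPlay it spawns a row of tiles, passing each its size and a reference back to the controller.
; When OnPlayerOverlapTile reports the second tile, the first tile jumps to the front and moves to the array's end.
; Once a moved tile reaches an X threshold, the world origin shifts to its X/Y location.
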(event Custom|OnPlayerOverlapTile
  (params (InTile :type BP%20Tile%20Object%20Reference))
  (if (== (Utilities|Array|FindItem (Variables|Default|GetTiles) InTile) 1)
    (CallFunction|MoveTailtoFront)))

(event EventBeginPlay
  (CallFunction|SpawnTiles))

(event Collision|EventActorBeginOverlap
  (params (OtherActor :type Actor%20Object%20Reference)))

(event EventTick
  (params (DeltaSeconds :type Float%20%28single-precision%29)))

(fn ConstructionScript)

(fn MoveTailtoFront
  (bind _tiles (Variables|Default|GetTiles))
  (if (Utilities|Array|IsValidIndex _tiles)
    (LocalVariables|SetTail (Utilities|Array|Get(acopy) _tiles))
    (Transformation|SetActorLocation (LocalVariables|GetTail) (+ (Transformation|GetActorLocation (LocalVariables|GetTail)) (Math|Vector|MakeVector (* (Variables|Default|GetTileHeight) (Variables|Default|GetTotalTileCount)) 0.0 0.0)) false false)
    (Utilities|Array|RemoveIndex (Variables|Default|GetTiles))
    (Utilities|Array|Add (Variables|Default|GetTiles) (LocalVariables|GetTail))
    (if (>= (.X (Math|Vector|BreakVector (Transformation|GetActorLocation (LocalVariables|GetTail)))) 1e+05)
      (Class|GameplayStatics|SetWorldOriginLocation (Utilities|Struct|MakeIntVector (Math|Float|Truncate (.X (Math|Vector|BreakVector (Transformation|GetActorLocation (LocalVariables|GetTail))))) (Math|Float|Truncate (.Y (Math|Vector|BreakVector (Transformation|GetActorLocation (LocalVariables|GetTail))))))))))

(fn SpawnTiles
  (for _index (range 0 (- (Variables|Default|GetTotalTileCount) 1))
    (bind _returnvalue (Game|SpawnActorfromClass "/Game/BP/BP_Tile.BP_Tile_C" (Math|Transform|MakeTransform (+ (Transformation|GetActorLocation) (Math|Vector|MakeVector (* (Variables|Default|GetTileHeight) _index) 0.0 0.0)) "0, 0, 0" "1.000000,1.000000,1.000000") "Undefined" "MultiplyWithRoot" 0 (Variables|Default|GetTileHeight) (Variables|Default|GetTileWidth) self 0))
    (Utilities|Array|Add (Variables|Default|GetTiles) _returnvalue)))