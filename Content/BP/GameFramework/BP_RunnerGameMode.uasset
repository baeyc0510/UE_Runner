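; BP_RunnerGameMode is the runner game mode that bootstraps a roguelite run through the RogueliteSubsystem.
; On BeginPlay it binds to the action-acquired event, registers each entry in its Actions collection with the subsystem, then starts the run.
; When a valid action is acquired, it prints the display name with a Korean "acquired!" suffix, ignoring stack counts.
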(event Custom|OnActionAcquired_Event
  (params (Action :type Roguelite%20Action%20Data%20Object%20Reference) (OldStacks :type Integer) (NewStacks :type Integer))
  (Utilities|IsValid Action
    (:Is%20Valid
      (Development|PrintString (Utilities|String|Append (Utilities|String|ToString(Text) (Variables|/Script/RogueliteCore.RogueliteActionData|GetDisplayName Action)) "획득!")))))

(event EventBeginPlay
  (bind _returnvalue (Subsystems|GetRogueliteSubsystem))
  (EventDispatchers|AssignOnActionAcquired (Subsystems|GetRogueliteSubsystem) (delegate Custom|OnActionAcquired_Event))
  (bind _result (Utilities|Set|ToArray (Variables|Default|GetActions)))
  (for _array_element _result
    (Class|RogueliteSubsystem|RegisterAction _returnvalue _array_element))
  (Class|RogueliteSubsystem|StartRun _returnvalue))

(event EventTick
  (params (DeltaSeconds :type Float%20%28single-precision%29)))

(fn ConstructionScript)