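; Actor that shows a floating damage number in the world through a widget component.
; On BeginPlay it casts the component's widget to W_FloatingWidget and picks white for normal or orange for critical hits.
; It then passes the damage amount and color to the widget, plays its floating animation, and sets its own lifespan so it removes itself.
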(event EventBeginPlay
  (bind _asw_floating_widget (Utilities|Casting|CastToW_FloatingWidget (UserInterface|GetWidget (Variables|Default|GetWidgetComp)))
    (:then
      (Variables|Default|SetWidgetInstance _asw_floating_widget)
      (Utilities|FlowControl|Sequence
        (:then_0
          (switch Utilities|FlowControl|Switch|SwitchonE_DamageType (Variables|Default|GetDamageType)
            (:NewEnumerator0
              (Variables|Default|SetDamageColor "(R=1.000000,G=1.000000,B=1.000000,A=1.000000)"))
            (:NewEnumerator1
              (Variables|Default|SetDamageColor "(R=1.000000,G=0.448528,B=0.026334,A=1.000000)"))))
        (:then_1
          (Default|InitWidget (Variables|Default|GetWidgetInstance) (Utilities|Text|ToText(Float) (Variables|Default|GetDamageAmount) "HalfToEven") (Variables|Default|GetDamageColor))
          (Default|PlayFloatingAnimation (Variables|Default|GetWidgetInstance)))
        (:then_2
          (Actor|SetLifeSpan (Variables|Default|GetDamageLifeTime)))))
    (:CastFailed
      (Development|PrintString "Invalid Damage Widget Class"))))

(event Collision|EventActorBeginOverlap
  (params (OtherActor :type Actor%20Object%20Reference)))

(event EventTick
  (params (DeltaSeconds :type Float%20%28single-precision%29)))

(fn ConstructionScript)