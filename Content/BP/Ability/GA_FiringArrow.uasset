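; Gameplay ability that fires an arrow from the avatar, gated by a cooldown.
; On activation it checks the cooldown, applies a cooldown effect, spawns BP_Arrow just in front of the avatar along its facing, then ends.
; Cooldown duration (base times coefficient) and arrow power come from RogueliteSubsystem run-state values, with the duration passed to the effect as a SetByCaller magnitude.
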(event Ability|EventActivateAbility
  (bind _returnvalue (Class|GameplayAbility|CheckAbilityCooldown))
  (if _returnvalue
    (CallFunction|CommitCooldown)
    (Development|PrintText "Fire!!")
    (CallFunction|FireArrow)
    (Ability|EndAbility)
    (else
      (Ability|EndAbility))))

(event Ability|EventOnEndAbility
  (params (bWasCancelled :type Boolean)))

(fn CommitCooldown
  (bind _returnvalue (Subsystems|GetRogueliteSubsystem))
  (bind _returnvalue_2 (Ability|GameplayEffect|AssignTagSetbyCallerMagnitude (Ability|MakeOutgoingGameplayEffectSpec "/Game/BP/Ability/GE_Cooldown_FiringArrow.GE_Cooldown_FiringArrow_C") "(TagName=\"Data.Cooldown\")" (* (Class|RogueliteSubsystem|GetRunStateValue _returnvalue "(TagName=\"Ability.FiringArrow.CooldownCoeff\")" 0.0) (Class|RogueliteSubsystem|GetRunStateValue _returnvalue "(TagName=\"Ability.FiringArrow.Cooldown\")" 0.0))))
  (Ability|ApplyGameplayEffectSpecToOwner _returnvalue_2))

(fn FireArrow
  (bind _returnvalue (Ability|GetAvatarActorfromActorInfo))
  (Game|SpawnActorfromClass "/Game/BP/Projectile/BP_Arrow.BP_Arrow_C" (Math|Transform|MakeTransform (+ (Transformation|GetActorLocation _returnvalue) (* (Transformation|GetActorForwardVector _returnvalue) 1e+02)) (Transformation|GetActorRotation _returnvalue)) "Undefined" "MultiplyWithRoot" 0 (Ability|GetAvatarActorfromActorInfo) (Class|RogueliteSubsystem|GetRunStateValue (Subsystems|GetRogueliteSubsystem) "(TagName=\"Ability.FiringArrow.Power\")" 0.0) 0))