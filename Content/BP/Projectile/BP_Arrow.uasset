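; BP_Arrow is an arrow projectile that delivers a Gameplay Ability System damage effect on overlap and expires after a short lifespan.
; When its capsule overlaps an actor other than the assigned SourceActor that implements CombatInterface, it builds a DamageEffect spec from the source's Ability System Component.
; It passes that spec to the target through an interface message, then destroys itself; other overlaps leave it intact.
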(event OnComponentBeginOverlap(Capsule)
  (params (OverlappedComponent :type Primitive%20Component%20Object%20Reference) (OtherActor :type Actor%20Object%20Reference) (OtherComp :type Primitive%20Component%20Object%20Reference) (OtherBodyIndex :type Integer) (bFromSweep :type Boolean) (SweepResult :type Hit%20Result%20Structure%20%28by%20ref%29))
  (CallFunction|HandleHitOtherActor OtherActor))

(event EventBeginPlay
  (Actor|SetLifeSpan 3.0))

(event Collision|EventActorBeginOverlap
  (params (OtherActor :type Actor%20Object%20Reference)))

(event EventTick
  (params (DeltaSeconds :type Float%20%28single-precision%29)))

(fn ConstructionScript)

(fn SetSourceActor
  (params (SourceActor :type Actor%20Object%20Reference))
  (Variables|Default|SetSourceActor SourceActor))

(fn HandleHitOtherActor
  (params (OtherActor :type Actor%20Object%20Reference))
  (bind _sourceactor (Variables|Default|GetSourceActor))
  (bind _returnvalue (Ability|GetAbilitySystemComponent _sourceactor))
  (if (!= (Variables|Default|GetSourceActor) OtherActor)
    (if (Utilities|DoesObjectImplementInterface OtherActor "/Script/Runner.CombatInterface")
      (Utilities|IsValid _returnvalue
        (:Is%20Valid
          (Class|CombatInterface|ApplyDamageEffect(Message) OtherActor (GameplayEffects|MakeOutgoingSpec _returnvalue (Variables|Default|GetDamageEffect) 0.0 (GameplayEffects|MakeEffectContext _returnvalue)))
          (Actor|DestroyActor))))))