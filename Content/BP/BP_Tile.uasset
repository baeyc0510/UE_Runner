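; BP_Tile is a level tile that spawns a BP_EnemyBase just above its origin on BeginPlay.
; The construction script scales the Cube from TileHeight, TileWidth and UnitExtent, and shapes the Box into a tall, thin trigger strip offset half the tile height along X.
; When a BP_ThirdPersonCharacter enters the Box, the tile passes itself to its TileController through OnPlayerOverlapTile, if that controller is valid.
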(event OnComponentBeginOverlap(Box)
  (params (OverlappedComponent :type Primitive%20Component%20Object%20Reference) (OtherActor :type Actor%20Object%20Reference) (OtherComp :type Primitive%20Component%20Object%20Reference) (OtherBodyIndex :type Integer) (bFromSweep :type Boolean) (SweepResult :type Hit%20Result%20Structure%20%28by%20ref%29))
  (Utilities|Casting|CastToBP_ThirdPersonCharacter OtherActor)
  (bind _tilecontroller (Variables|Default|GetTileController)
    (:then
      (Default|OnPlayerOverlapTile _tilecontroller self))
    (:else)))

(event EventBeginPlay
  (Game|SpawnActorfromClass "/Game/BP/Characters/Enemy/BP_EnemyBase.BP_EnemyBase_C" (Math|Transform|MakeTransform (+ (Transformation|GetActorLocation) "0.000000,0.000000,50.000000") (Transformation|GetActorRotation)) "Undefined" "MultiplyWithRoot" 0 0))

(event Collision|EventActorBeginOverlap
  (params (OtherActor :type Actor%20Object%20Reference)))

(event EventTick
  (params (DeltaSeconds :type Float%20%28single-precision%29)))

(fn ConstructionScript
  (bind _unitextent (Variables|Default|GetUnitExtent))
  (bind _returnvalue (/ _unitextent 2.0))
  (Transformation|SetRelativeScale3D (Variables|Default|GetCube) (Math|Vector|MakeVector (/ (Variables|Tile|GetTileHeight) (Variables|Default|GetUnitExtent)) (/ (Variables|Tile|GetTileWidth) (Variables|Default|GetUnitExtent)) 0.25))
  (Components|Box|SetBoxExtent (Variables|Default|GetBox) (Math|Vector|MakeVector _returnvalue _returnvalue 3e+02) true)
  (Transformation|SetRelativeScale3D (Variables|Default|GetBox) (Math|Vector|MakeVector (/ (/ (Variables|Tile|GetTileHeight) (Variables|Default|GetUnitExtent)) 1e+01) (/ (Variables|Tile|GetTileWidth) (Variables|Default|GetUnitExtent)) 1.0))
  (Transformation|SetRelativeLocation (Variables|Default|GetBox) (Math|Vector|MakeVector (/ (Variables|Tile|GetTileHeight) 2.0) 0.0 0.0) false false))