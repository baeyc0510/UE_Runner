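; BP_Tile is a level tile that notifies its TileController when the third-person character crosses its trigger.
; The construction script scales the cube from TileHeight, TileWidth and UnitExtent, and places a thin, tile-wide trigger box half the tile height along X.
; Overlapping that box passes the tile to the controller's OnPlayerOverlapTile.
; Getter functions return unit-scale transforms for boss, left and right spawn points.
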(event OnComponentBeginOverlap(Box)
  (params (OverlappedComponent :type Primitive%20Component%20Object%20Reference) (OtherActor :type Actor%20Object%20Reference) (OtherComp :type Primitive%20Component%20Object%20Reference) (OtherBodyIndex :type Integer) (bFromSweep :type Boolean) (SweepResult :type Hit%20Result%20Structure%20%28by%20ref%29))
  (Utilities|Casting|CastToBP_ThirdPersonCharacter OtherActor)
  (bind _tilecontroller (Variables|Default|GetTileController)
    (:then
      (Default|OnPlayerOverlapTile _tilecontroller self))
    (:else)))

(event EventBeginPlay)

(event Collision|EventActorBeginOverlap
  (params (OtherActor :type Actor%20Object%20Reference)))

(event EventTick
  (params (DeltaSeconds :type Float%20%28single-precision%29)))

(fn ConstructionScript
  (bind _unitextent (Variables|Default|GetUnitExtent))
  (bind _returnvalue (/ _unitextent 2.0))
  (Transformation|SetRelativeScale3D (Variables|Default|GetCube) (Math|Vector|MakeVector (/ (Variables|Tile|GetTileHeight) (Variables|Default|GetUnitExtent)) (/ (Variables|Tile|GetTileWidth) (Variables|Default|GetUnitExtent)) 0.25))
  (Components|Box|SetBoxExtent (Variables|Default|GetBox) (Math|Vector|MakeVector _returnvalue _returnvalue 3e+02) true)
  (Transformation|SetRelativeScale3D (Variables|Default|GetBox) (Math|Vector|MakeVector (/ (/ (Variables|Tile|GetTileHeight) (Variables|Default|GetUnitExtent)) 1e+01) (/ (Variables|Tile|GetTileWidth) (Variables|Default|GetUnitExtent)) 1.0))
  (Transformation|SetRelativeLocation (Variables|Default|GetBox) (Math|Vector|MakeVector (/ (Variables|Tile|GetTileHeight) 2.0) 0.0 0.0) false false))

(fn GetBossSpawnTransform
  (bind _spawnpoint_boss (Variables|Default|GetSpawnPoint_Boss))
  (bind _returnvalue (Transformation|GetWorldTransform _spawnpoint_boss))
  (bind (_location _rotation) (Math|Transform|BreakTransform _returnvalue))
  (return (Math|Transform|MakeTransform _location _rotation)))

(fn GetLeftSpawnTransform
  (bind _spawnpoint_left (Variables|Default|GetSpawnPoint_Left))
  (bind _returnvalue (Transformation|GetWorldTransform _spawnpoint_left))
  (bind (_location _rotation) (Math|Transform|BreakTransform _returnvalue))
  (return (Math|Transform|MakeTransform _location _rotation)))

(fn GetRightSpawnTransform
  (bind _spawnpoint_right (Variables|Default|GetSpawnPoint_Right))
  (bind _returnvalue (Transformation|GetWorldTransform _spawnpoint_right))
  (bind (_location _rotation) (Math|Transform|BreakTransform _returnvalue))
  (return (Math|Transform|MakeTransform _location _rotation)))