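; BP_SpawnManager spawns enemies and clears them in groups by spawn key.
; SpawnEnemy creates a BP_EnemyBase at the left transform (the right one is unused) and records it in SpawnedActors, a map of key to STSpawnPool actor array.
; DestorySpawnedActorsByKey destroys that key's valid actors in reverse order and removes the entry.
; SpawnBoss spawns the same BP_EnemyBase class without tracking it, so key-based cleanup does not reach it.
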(event EventBeginPlay)

(event EventTick
  (params (DeltaSeconds :type Float%20%28single-precision%29)))

(fn SpawnEnemy
  (params (SpawnKey :type Name) (LeftSpawnTransform :type Transform) (RightSpawnTransform :type Transform))
  (bind _spawnedactors (Variables|Default|GetSpawnedActors))
  (bind (_value _returnvalue) (Utilities|Map|Find _spawnedactors SpawnKey))
  (bind _returnvalue_2 (Game|SpawnActorfromClass "/Game/BP/Characters/Enemy/BP_EnemyBase.BP_EnemyBase_C" LeftSpawnTransform "Undefined" "MultiplyWithRoot" 0 0))
  (Utilities|FlowControl|Sequence
    (:then_0
      (if _returnvalue
        (bind _output_get (LocalVariables|SetPool _value))
        (Utilities|Array|Add (Utilities|Struct|BreakST_SpawnPool _output_get) _returnvalue_2)
        (else
          (LocalVariables|SetPool (Utilities|Struct|MakeST_SpawnPool (Utilities|Array|MakeArray _returnvalue_2))))))
    (:then_1
      (Utilities|Map|Add (Variables|Default|GetSpawnedActors) SpawnKey (LocalVariables|GetPool)))))

(fn SpawnBoss
  (params (SpawnTransform :type Transform))
  (Game|SpawnActorfromClass "/Game/BP/Characters/Enemy/BP_EnemyBase.BP_EnemyBase_C" SpawnTransform "Undefined" "MultiplyWithRoot" 0 0))

(fn DestorySpawnedActorsbyKey
  (params (SpawnKey :type Name))
  (bind _spawnedactors (Variables|Default|GetSpawnedActors))
  (bind (_value _returnvalue) (Utilities|Map|Find _spawnedactors SpawnKey))
  (if _returnvalue
    (bind _arrayelement (Utilities|Array|ReverseforEachLoop (Utilities|Struct|BreakST_SpawnPool _value))
      (:LoopBody
        (Utilities|IsValid _arrayelement
          (:Is%20Valid
            (Actor|DestroyActor _arrayelement))))
      (:Completed
        (Utilities|Map|Remove (Variables|Default|GetSpawnedActors) SpawnKey)))))